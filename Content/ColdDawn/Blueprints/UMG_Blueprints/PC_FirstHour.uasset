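; PC_FirstHour is a Blueprint that toggles the pause menu in the game when the Pause input action is pressed.
; It creates UMG_MainMenu, switches to game-and-UI input with a visible cursor, pauses the game and turns off the Character_FirstHourUMG HUD.
; A stored widget reference serves as the toggle state, so the next press removes the menu, clears the reference and restores gameplay input, cursor and HUD.
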(event Input|ActionEvents|InputActionPause
  (params (Key :type Key%20Structure :default "None"))
  (bind _returnvalue (Game|GetPlayerController 0))
  (bind _returnvalue_2 (Game|GetPlayerController 0))
  (:Pressed
    (Utilities|IsValid (Variables|Default|GetPauseUIRef)
      (:Is%20Valid
        (Widget|RemovefromParent (Variables|Default|GetPauseUIRef))
        (Variables|Default|SetPauseUIRef 0)
        (Input|SetInputModeGameOnly _returnvalue)
        (Variables|/Script/Engine.PlayerController|SetbShowMouseCursor _returnvalue false)
        (Game|SetGamePaused false)
        (Default|ToggleHudON (.AsCharacter%20First%20Hour%20UMG (Utilities|Casting|CastToCharacter_FirstHourUMG (Game|GetPlayerCharacter 0)))))
      (:Is%20Not%20Valid
        (bind _returnvalue_3 (UserInterface|CreateWidget "/Game/FirstHourUMG/Widgets/UMG_MainMenu.UMG_MainMenu_C"))
        (bind _output_get (Variables|Default|SetPauseUIRef _returnvalue_3))
        (UserInterface|Viewport|AddtoViewport _output_get 0)
        (Input|SetInputModeGameandUI _returnvalue_2 0 "DoNotLock" true)
        (Variables|/Script/Engine.PlayerController|SetbShowMouseCursor _returnvalue_2 true)
        (Game|SetGamePaused true)
        (Default|ToggleHudOff (.AsCharacter%20First%20Hour%20UMG (Utilities|Casting|CastToCharacter_FirstHourUMG (Game|GetPlayerCharacter 0))))))))

(fn ConstructionScript)