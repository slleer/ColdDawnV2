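; Door actor that swings a door mesh around its yaw axis in response to the E key.
; Both pressing and releasing E flip an Open flag, so each change lasts only while the key is held.
; Tick polls the flag to play or reverse a timeline, whose track sets the door's relative rotation.
; An overlap check for the player character in the Box is left unconnected, so proximity does not gate input.
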(event EventTick
  (params (DeltaSeconds :type Float%20%28single-precision%29))
  (if (Variables|Default|GetOpen)
    (bind _newtrack_0 (Timeline|OpenAndCloseDoor Play)
      (:Update
        (Transformation|SetRelativeRotation (Variables|Default|GetDoor) (Math|Rotator|MakeRotator 0.0 0.0 _newtrack_0) false false)))
    (else
      (Timeline|OpenAndCloseDoor Reverse))))

(event Input|KeyboardEvents|E
  (params (Key :type Key%20Structure :default "None"))
  (:Pressed
    (Variables|Default|SetOpen (not (Variables|Default|GetOpen))))
  (:Released
    (Variables|Default|SetOpen (not (Variables|Default|GetOpen)))))

(fn ConstructionScript)